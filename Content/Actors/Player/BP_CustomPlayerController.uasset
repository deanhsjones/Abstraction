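; Player controller that handles movement, camera look and a double jump for the player character.
; Axis inputs move the controlled Character along its forward and right vectors and feed yaw and pitch.
; Jump calls the normal jump when not falling; while falling, a DoN allows one upward launch that overrides Z velocity, resetting on the next non-falling jump.
; The falling check and launch find BP_CustomPlayerCharacter via GetActorOfClass, not the controlled pawn.
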(event `InputAction|Jump`
  (params (Key :type "Key Structure"))
  (:`Pressed`
    (bind _returnvalue (`GameplayStatics.GetActorOfClass` "/Game/Actors/Player/BP_CustomPlayerCharacter.BP_CustomPlayerCharacter_C"))
    (if (`NavMovementComponent.IsFalling` (`Character.CharacterMovement` _returnvalue))
      (`/Engine/EditorBlueprintResources/StandardMacros.Do N` 1 :!label _label
        (:`Exit`
          (bind _returnvalue_2 (`GameplayStatics.GetActorOfClass` "/Game/Actors/Player/BP_CustomPlayerCharacter.BP_CustomPlayerCharacter_C"))
          (`Character.LaunchCharacter` _returnvalue_2 (0.0 0.0 600.0) false true)))
      (else
        (bind _ascharacter (cast `Character` (`self.K2_GetPawn`)))
        (`Character.Jump` _ascharacter)
        (goto _label :!via `Reset`)))))

(event `InputAxis|MoveForward`
  (params (AxisValue :type "Float (single-precision)"))
  (bind _ascharacter (cast `Character` (`self.K2_GetPawn`)))
  (`PawnMovementComponent.AddInputVector` (`Pawn.GetMovementComponent` _ascharacter) (* (`self.GetActorForwardVector` _ascharacter) AxisValue) false))

(event `InputAxis|MoveRight`
  (params (AxisValue :type "Float (single-precision)"))
  (bind _ascharacter (cast `Character` (`self.K2_GetPawn`)))
  (`PawnMovementComponent.AddInputVector` (`Pawn.GetMovementComponent` _ascharacter) (* (`self.GetActorRightVector` _ascharacter) AxisValue) false))

(event `InputAxis|Turn`
  (params (AxisValue :type "Float (single-precision)"))
  (`self.AddYawInput` AxisValue))

(event `InputAxis|LookUp`
  (params (AxisValue :type "Float (single-precision)"))
  (`self.AddPitchInput` AxisValue))

(fn `UserConstructionScript`)