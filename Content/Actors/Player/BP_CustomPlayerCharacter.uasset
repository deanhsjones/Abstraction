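; Player character Blueprint that handles crouching and holds unfinished camera-perspective switching.
; Left Ctrl crouches by squashing the actor to half height and applying crouched walk speed, then restores both on release.
; Landing clears a jump-reset flag.
; Helper graphs toggle cameras between third-person, first-person and over-the-shoulder views, but the selection logic cycling them is disconnected and the OTS-to-TPP graph is empty.
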(event `Key|V`
  (params (Key :type "Key Structure")))

(event `Key|LeftControl`
  (params (Key :type "Key Structure"))
  (bind _charactermovement (`self.CharacterMovement`))
  (:`Pressed`
    (`self.Crouch`)
    (`self.SetActorScale3D` (1.0 1.0 0.5))
    (set `CharacterMovementComponent.MaxWalkSpeed` (`CharacterMovementComponent.MaxWalkSpeedCrouched` _charactermovement) _charactermovement))
  (:`Released`
    (`self.UnCrouch`)
    (`self.SetActorScale3D` (1.0 1.0 1.0))
    (set `CharacterMovementComponent.MaxWalkSpeed` (`self.Walk Speed`) (`self.CharacterMovement`))))

(event `self.OnLanded`
  (params (Hit :type "HitResult Structure (by ref)"))
  (set `self.resetJump` false))

(fn `UserConstructionScript`)